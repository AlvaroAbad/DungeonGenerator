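; Demo camera that circles a DungeonMapper's dungeon and periodically regenerates it as a showcase.
; On BeginPlay it moves to the mapper, sizes its spring arm from the NavMeshBoundsVolume extent, then generates and renders the first dungeon.
; Tick yaws the actor at RotationSpeed, and a looping timer clears, regenerates and renders a new dungeon every half turn.
; An unconnected MultiGate for hiding hallways never runs.
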(event Custom|NextStep
  (Class|DungeonMapper|ClearAll (Variables|Default|GetDungeonGenerator))
  (Class|DungeonMapper|GenerateDungeonRooms (Variables|Default|GetDungeonGenerator))
  (Class|DungeonMapper|RenderDungeon (Variables|Default|GetDungeonGenerator)))

(event EventBeginPlay
  (bind _returnvalue (Actor|GetActorOfClass "/Script/DungeonGenerator.DungeonMapper"))
  (Variables|Default|SetDungeonGenerator _returnvalue)
  (Transformation|SetActorLocation self (Transformation|GetActorLocation _returnvalue) false true)
  (bind _returnvalue_2 (Actor|GetActorOfClass "/Script/NavigationSystem.NavMeshBoundsVolume"))
  (Variables|/Script/Engine.SpringArmComponent|SetTargetArmLength (Variables|Default|GetSpringArm) (+ (Math|Vector|VectorLength (.BoxExtent (Collision|GetActorBounds _returnvalue_2 false false))) 1e+03))
  (Utilities|Time|SetTimerbyEvent (delegate Custom|NextStep) (/ 1.8e+02 (Variables|Default|GetRotationSpeed)) true)
  (Class|DungeonMapper|ClearAll (Variables|Default|GetDungeonGenerator))
  (Class|DungeonMapper|GenerateDungeonRooms (Variables|Default|GetDungeonGenerator))
  (Class|DungeonMapper|RenderDungeon (Variables|Default|GetDungeonGenerator)))

(event Collision|EventActorBeginOverlap
  (params (OtherActor :type Actor%20Object%20Reference)))

(event EventTick
  (params (DeltaSeconds :type Float%20%28single-precision%29))
  (Class|Actor|AddActorWorldRotation (Math|Rotator|MakeRotator 0.0 0.0 (* DeltaSeconds (Variables|Default|GetRotationSpeed)))))

(fn ConstructionScript)